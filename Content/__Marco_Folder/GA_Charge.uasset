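; GA_Charge is a Gameplay Ability for a hold-and-release charge that launches the avatar forward and upward.
; On input release, the clamped hold time scales both strength and duration of a root motion constant force.
; When the force finishes, it polls player 0's movement every 0.1 seconds and ends the ability once not falling.
; CommitAbility and montage playback are present but disconnected, and ending prints a debug string.
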(event Ability|EventActivateAbility
  (bind _returnvalue (Ability|GetAvatarActorfromActorInfo))
  (bind _returnvalue_2 (Transformation|GetActorForwardVector _returnvalue))
  (bind _timeheld (Ability|Tasks|WaitInputRelease false)
    (:OnRelease
      (Ability|Tasks|ApplyRootMotionConstantForce "None" (Math|Vector|MakeVector (.x _returnvalue_2) (.y _returnvalue_2) (.z (Transformation|GetActorUpVector _returnvalue))) (* (Math|Float|Max(Float) (Math|Float|Min(Float) _timeheld 5.0) 1.0) 5e+02) (* (Math|Float|Max(Float) (Math|Float|Min(Float) _timeheld 5.0) 1.0) 0.15) false 0 "MaintainLastRootMotionVelocity"
        (:OnFinish
          (if (not (AI|Components|NavMovement|IsFalling (Variables|/Script/Engine.Character|GetCharacterMovement (Game|GetPlayerCharacter 0)))) :!label _label
            (Ability|EndAbility)
            (else
              (Utilities|FlowControl|Delay 0.1)
              (goto _label))))))))

(event Ability|EventOnEndAbility
  (params (bWasCancelled :type Boolean))
  (Development|PrintString "Ability_End"))