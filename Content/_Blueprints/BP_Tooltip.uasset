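; BP_Tooltip is a trigger volume that shows an on-screen tooltip while the hero is inside its box.
; When a BP_Hero begins overlapping, it creates a WB_ToolTip widget, passes in its ToolTipText and adds it to the viewport.
; A DoOnce prevents repeat creation until the hero's end overlap removes the widget and resets the gate.
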(event OnComponentBeginOverlap(Box)
  (params (OverlappedComponent :type Primitive%20Component%20Object%20Reference) (OtherActor :type Actor%20Object%20Reference) (OtherComp :type Primitive%20Component%20Object%20Reference) (OtherBodyIndex :type Integer) (bFromSweep :type Boolean) (SweepResult :type Hit%20Result%20Structure%20%28by%20ref%29))
  (Utilities|Casting|CastToBP_Hero OtherActor)
  (Utilities|FlowControl|DoOnce false
    (:Completed
      (bind _returnvalue (UserInterface|CreateWidget "/Game/_UI/WB_ToolTip.WB_ToolTip_C"))
      (bind _output_get (Variables|Default|SetWidgetRef _returnvalue))
      (Variables|/Game/_UI/WB_ToolTip.WB_ToolTip_C|SetToolTipTextToDisplay _output_get (Variables|Default|GetTool%20Tip%20Text))
      (UserInterface|Viewport|AddtoViewport _output_get 0))))

(event OnComponentEndOverlap(Box)
  (params (OverlappedComponent :type Primitive%20Component%20Object%20Reference) (OtherActor :type Actor%20Object%20Reference) (OtherComp :type Primitive%20Component%20Object%20Reference) (OtherBodyIndex :type Integer))
  (Utilities|Casting|CastToBP_Hero OtherActor)
  (Widget|RemovefromParent (Variables|Default|GetWidgetRef))
  (Utilities|FlowControl|DoOnce false) ; enters at Reset
)

(fn ConstructionScript)