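; BP_GravityZone is a volume that changes the hero's gravity scale while the hero is inside its cube.
; Overlap starts a looping timer that applies the zone's GravityZoneScale whenever BP_Hero uses neither jetpack nor dive.
; Leaving resets gravity to normal and clears the Loop flag, which idles the timer's logic without clearing the timer.
; The construction script tints the cube through a dynamic instance of M_Gravity.
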(event OnComponentBeginOverlap(Cube)
  (params (OverlappedComponent :type Primitive%20Component%20Object%20Reference) (OtherActor :type Actor%20Object%20Reference) (OtherComp :type Primitive%20Component%20Object%20Reference) (OtherBodyIndex :type Integer) (bFromSweep :type Boolean) (SweepResult :type Hit%20Result%20Structure%20%28by%20ref%29))
  (bind _asbp_hero (Utilities|Casting|CastToBP_Hero OtherActor))
  (bind _output_get (Variables|Default|SetBP%20Hero%20Ref _asbp_hero))
  (bind _output_get_2 (Variables|Default|SetLoop? true))
  (Utilities|Time|SetTimerbyEvent (delegate Custom|Activate%20Gravity%20Zone) 0.1 _output_get_2))

(event OnComponentEndOverlap(Cube)
  (params (OverlappedComponent :type Primitive%20Component%20Object%20Reference) (OtherActor :type Actor%20Object%20Reference) (OtherComp :type Primitive%20Component%20Object%20Reference) (OtherBodyIndex :type Integer))
  (Utilities|Casting|CastToBP_Hero OtherActor)
  (Variables|/Script/Engine.CharacterMovementComponent|SetGravityScale (Variables|/Script/Engine.Character|GetCharacterMovement (stale OnComponentBeginOverlap(Cube) _output_get)) 1.0)
  (Variables|Default|SetLoop? false))

(event Custom|Activate%20Gravity%20Zone
  (bind _bp_hero_ref (Variables|Default|GetBP%20Hero%20Ref))
  (if (Variables|Default|GetLoop?)
    (if (Math|Boolean|NORBoolean (Variables|/Game/_Blueprints/BP_Hero.BP_Hero_C|GetIsUsingJetpack? _bp_hero_ref) (Variables|/Game/_Blueprints/BP_Hero.BP_Hero_C|GetIsUsingDive? _bp_hero_ref))
      (Variables|/Script/Engine.CharacterMovementComponent|SetGravityScale (Variables|/Script/Engine.Character|GetCharacterMovement (stale OnComponentBeginOverlap(Cube) _output_get)) (Variables|Default|GetGravity%20Zone%20Scale)))))

(fn ConstructionScript
  (bind _returnvalue (Rendering|Material|CreateDynamicMaterialInstance (Variables|Default|GetCube) 0 "/Game/_Materials/M_Gravity.M_Gravity" "None" :!class /Script/Engine.PrimitiveComponent))
  (Rendering|Material|SetVectorParameterValue _returnvalue "Color" (Variables|Default|GetValue) :!class /Script/Engine.MaterialInstanceDynamic))