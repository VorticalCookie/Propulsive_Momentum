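; BP_RollingLog is a physics-driven rolling log hazard that kills actors it touches.
; Shortly after BeginPlay, it launches its Cylinder along that component's right vector with a velocity-change impulse scaled by Speed.
; On Cylinder overlap, it waits a tick, then applies Damage through the other actor's AC_Health component, if present, and calls death directly.
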(event OnComponentBeginOverlap(Cylinder)
  (params (OverlappedComponent :type Primitive%20Component%20Object%20Reference) (OtherActor :type Actor%20Object%20Reference) (OtherComp :type Primitive%20Component%20Object%20Reference) (OtherBodyIndex :type Integer) (bFromSweep :type Boolean) (SweepResult :type Hit%20Result%20Structure%20%28by%20ref%29))
  (bind _returnvalue (Actor|GetComponentbyClass OtherActor "/Game/__Benjamin_Folder/AC_Health.AC_Health_C"))
  ;[0.15 0.15 0.15 0.5] Call Death
  (Utilities|FlowControl|DelayUntilNextTick)
  (Utilities|IsValid _returnvalue
    (:Is%20Valid
      (Default|TakeDamage _returnvalue (Variables|Default|GetDamage))
      (Default|CallDeath _returnvalue))))

(event EventBeginPlay
  (bind _cylinder (Variables|Default|GetCylinder))
  (Utilities|FlowControl|Delay 0.2)
  (Physics|AddImpulse _cylinder (* (Math|Vector|GetRightVector _cylinder) (Variables|Default|GetSpeed)) "None" true))

(fn ConstructionScript)